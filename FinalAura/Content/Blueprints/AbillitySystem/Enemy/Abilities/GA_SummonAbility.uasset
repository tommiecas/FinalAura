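; Gameplay ability that summons random enemy minions around the caster, using the Goblin Shaman summon montage.
; It shuffles the computed spawn locations and shows a ground-summon Niagara effect at each, then plays the montage.
; On the montage's gameplay event, a delayed loop spawns AI-controlled minions one at a time, facing away from the caster.
; Each spawn increments the caster's minion count, and a destroy binding decrements it.
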(event Custom|OnDestroyed_Event
  (params (DestroyedActor :type Actor%20Object%20Reference))
  (Class|CombatInterface|SetMinionCount(Message) (Ability|GetAvatarActorfromActorInfo) -1))

(event Ability|EventActivateAbility
  (bind _returnvalue (Class|AuraSummonAbility|GetSpawnLocations))
  (bind _output_get (Variables|Default|SetSpawnLocations _returnvalue))
  (Utilities|Array|Shuffle _output_get)
  (for _array_element _output_get
    (Niagara|SpawnSystematLocation "/Game/Assets/Effects/Combat/NS_GroundSummon.NS_GroundSummon" _array_element))
  (|PlayMontageandWaitProxy "None" "/Game/Blueprints/Characters/Enemies/Goblins/Goblin_Shamans/AnimationMontages/AM_GoblinShaman_Summon.AM_GoblinShaman_Summon" 1.0 "None" true 1.0 0.0 false
    (:then
      (Ability|Tasks|WaitGameplayEvent "(TagName=\"Montage.Attack.1\")" 0
        (:EventReceived
          (if (< (Variables|Default|GetSpawnLocationIndex) (Utilities|Array|Length (Variables|Default|GetSpawnLocations))) :!label _label
            (bind _returnvalue_2 (Game|SpawnActorfromClass (Class|AuraSummonAbility|GetRandomMinionClass) (Math|Transform|MakeTransform (+ (Utilities|Array|Get(acopy) (Variables|Default|GetSpawnLocations) (Variables|Default|GetSpawnLocationIndex)) "0.000000,0.000000,70.000000") (Math|Rotator|FindLookatRotation (Transformation|GetActorLocation (Ability|GetAvatarActorfromActorInfo)) (+ (Utilities|Array|Get(acopy) (Variables|Default|GetSpawnLocations) (Variables|Default|GetSpawnLocationIndex)) "0.000000,0.000000,70.000000")) "1.000000,1.000000,1.000000") "AlwaysSpawn" "MultiplyWithRoot" 0 0))
            (Game|AssignOnDestroyed _returnvalue_2 (delegate Custom|OnDestroyed_Event))
            (Pawn|SpawnDefaultController _returnvalue_2)
            (Class|CombatInterface|SetMinionCount(Message) (Ability|GetAvatarActorfromActorInfo) 1)
            (Math|Integer|IncrementInt (Variables|Default|GetSpawnLocationIndex)
              (:%20%20
                (Utilities|FlowControl|Delay 0.2)
                (goto _label)))))))))